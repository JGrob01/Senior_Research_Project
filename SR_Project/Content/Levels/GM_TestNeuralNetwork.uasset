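; Game mode that runs neural-network AI trials, training the agent across repeated level reloads toward a goal.
; On save check, it initializes the AI, restores its four move/jump networks from a SaveGame, passes the goal location and starts timers.
; Timeout or death triggers backprop, a final AI save and level reload.
; Times and reset counts persist in the GameInstance and are written to file on level change.
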(event `self.ReceiveBeginPlay`
  ;[1 1 1 1 32] BEGIN PLAY
  (bind _asbp_game_instance (cast `/Game/Data/BP_GameInstance` (`GameplayStatics.GetGameInstance`)))
  (bind _output_get (set `self.GameInstanceRef` _asbp_game_instance))
  (set `self.Neural Network Test` (`/Game/Data/BP_GameInstance.networkInUse` _output_get))
  (`KismetSystemLibrary.PrintString` "Gamemode Spawn"))

(event `LevelTimer`
  (bind _gameinstanceref (`self.GameInstanceRef`))
  (bind (_leveldata_neuralnetworktype _leveldata_totaltimetocompletelevel _leveldata_timetocompletelevel _leveldata_totalattemptstocompletelevel _leveldata_numberofresetsbytime _leveldata_numberofresetsbydeath) (break `/Game/Data/DataCollection/S_PerLevelData` (`/Game/Data/BP_GameInstance.LevelData` _gameinstanceref)))
  ;[1 1 1 1 32] LEVEL DATA AND STATISTICS
  (`|ExecutionSequence`
    (:`then_0`
      (bind (_direction _leveltime) (`Timeline|LevelTimeLine` :`NewTime` _leveldata_totaltimetocompletelevel :!via `SetNewTime` :!label _label)
        (:`Update`
          (set `/Game/Data/BP_GameInstance.LevelData` (make `/Game/Data/DataCollection/S_PerLevelData` _leveldata_neuralnetworktype _leveltime _leveldata_timetocompletelevel _leveldata_totalattemptstocompletelevel _leveldata_numberofresetsbytime _leveldata_numberofresetsbydeath) _gameinstanceref))))
    (:`then_1`
      (goto _label))))

(event `BeginTrial`
  ;[1 1 1 1 32] TRIAL LOGIC
  ;;[1 1 1 1 24] BEGIN AND RESTART
  (`KismetSystemLibrary.K2_SetTimerDelegate` (delegate `RestartTrial`) 30.0 true)
  (`/Game/AI/BP_AICharacter.RunNNTrial` (`self.AI`))
  (`self.LevelTimer`)
  (`self.TrialTimer`))

(event `CheckSaveGame`
  (params (AI :type "/Game/AI/BP_AICharacter Object Reference"))
  ;[1 1 1 1 32] SAVE AND LOAD FUNCTIONS
  ;;[1 1 1 1 24] CHECK IF SAVE GAME EXISTS:
  ;; IF SO SEND IT TO THE AI
  ;; ELSE CREATE A NEW SAVE
  (bind _output_get (set `self.AI` AI))
  (bind _returnvalue (`GameplayStatics.DoesSaveGameExist` "save1"))
  (if _returnvalue
    (`/Game/AI/BP_AICharacter.InitializeAI` _output_get (`self.Neural Network Test`))
    (`self.LoadNeuralNetworks`)
    (else
      (bind _returnvalue_2 (`GameplayStatics.CreateSaveGameObject` "/Game/Data/BP_SaveGame.BP_SaveGame_C"))
      (bind _output_get_2 (set `self.SaveGameRef` _returnvalue_2))
      (`GameplayStatics.SaveGameToSlot` _output_get_2 "save1")
      (`/Game/AI/BP_AICharacter.InitializeAI` _output_get (`self.Neural Network Test`))))
  (`self.GiveInfoToAI`)
  (`self.BeginTrial`))

(event `RestartTrial`
  (bind _ai (`self.AI`))
  ;[1 1 1 1 32] TRIAL LOGIC
  ;;[1 1 1 1 24] BEGIN AND RESTART
  (`self.AddAttemptByTime`)
  (`/Game/AI/BP_AICharacter.BackProp` _ai)
  (`/Game/AI/BP_AICharacter.FinalSaveBeforeReset` _ai :!label _label_2)
  (bind _returnvalue (`GameplayStatics.GetCurrentLevelName` true))
  (`GameplayStatics.OpenLevel` (`KismetStringLibrary.Conv_StringToName` _returnvalue)))

(event `DeathRestart`
  ;[1 1 1 1 32] TRIAL LOGIC
  ;;[1 1 1 1 24] BEGIN AND RESTART
  (`self.AddAttemptByDeath`)
  (`/Game/AI/BP_AICharacter.BackpropFromDeath` (`self.AI`))
  (goto _label_2))

(event `TrialTimer`
  (bind _gameinstanceref (`self.GameInstanceRef`))
  (bind (_leveldata_neuralnetworktype _leveldata_totaltimetocompletelevel _leveldata_timetocompletelevel _leveldata_totalattemptstocompletelevel _leveldata_numberofresetsbytime _leveldata_numberofresetsbydeath) (break `/Game/Data/DataCollection/S_PerLevelData` (`/Game/Data/BP_GameInstance.LevelData` _gameinstanceref)))
  ;[1 1 1 1 32] LEVEL DATA AND STATISTICS
  (bind (_direction _leveltime) (`Timeline|Timeline`)
    (:`Update`
      (set `/Game/Data/BP_GameInstance.LevelData` (make `/Game/Data/DataCollection/S_PerLevelData` _leveldata_neuralnetworktype _leveldata_totaltimetocompletelevel _leveltime _leveldata_totalattemptstocompletelevel _leveldata_numberofresetsbytime _leveldata_numberofresetsbydeath) _gameinstanceref))))

(event `GiveInfoToAI`
  ;[1 1 1 1 32] SAVE AND LOAD FUNCTIONS
  ;;[1 1 1 1 24] CHECK IF SAVE GAME EXISTS:
  ;; IF SO SEND IT TO THE AI
  ;; ELSE CREATE A NEW SAVE
  (bind _outactors (`GameplayStatics.GetAllActorsOfClass` "/Game/Objects/Interactables/BP_Goal.BP_Goal_C"))
  (for _array_element _outactors
    _)
  (`/Game/AI/BP_AICharacter.setGoalLocation` (`self.AI`) (`self.K2_GetActorLocation` _array_element)))

(event `GoToNextLevel`
  (params (nextLevel :type String))
  ;[1 1 1 1 32] TRIAL LOGIC
  ;;[1 1 1 1 24] GO TO NEXT LEVEL
  (`/Game/AI/BP_AICharacter.FinalSaveBeforeReset` (`self.AI`))
  (`self.SaveDataToFile`)
  (`GameplayStatics.OpenLevel` (`KismetStringLibrary.Conv_StringToName` nextLevel)))

(event `AddAttemptByDeath`
  (bind _gameinstanceref (`self.GameInstanceRef`))
  (bind (_leveldata_neuralnetworktype _leveldata_totaltimetocompletelevel _leveldata_timetocompletelevel _leveldata_totalattemptstocompletelevel _leveldata_numberofresetsbytime _leveldata_numberofresetsbydeath) (break `/Game/Data/DataCollection/S_PerLevelData` (`/Game/Data/BP_GameInstance.LevelData` _gameinstanceref)))
  ;[1 1 1 1 32] LEVEL DATA AND STATISTICS
  (set `/Game/Data/BP_GameInstance.LevelData` (make `/Game/Data/DataCollection/S_PerLevelData` _leveldata_neuralnetworktype _leveldata_totaltimetocompletelevel _leveldata_timetocompletelevel (+ _leveldata_totalattemptstocompletelevel 1) _leveldata_numberofresetsbytime (+ _leveldata_numberofresetsbydeath 1)) _gameinstanceref))

(event `LoadNeuralNetworks`
  (bind _ai (`self.AI`))
  (bind _savegameref (`self.SaveGameRef`))
  (bind _nn_move_right (`/Game/AI/BP_AICharacter.NN_Move_Right` _ai))
  (bind _nn_jump_right (`/Game/AI/BP_AICharacter.NN_Jump_Right` _ai))
  (bind _nn_move_left (`/Game/AI/BP_AICharacter.NN_Move_Left` _ai))
  (bind _nn_jump_left (`/Game/AI/BP_AICharacter.NN_Jump_Left` _ai))
  ;[1 1 1 1 32] SAVE AND LOAD FUNCTIONS
  ;;[1 1 1 1 24] LOAD THE SAVE DATA AND SEND IT TO THE AI
  (bind _returnvalue (`GameplayStatics.LoadGameFromSlot` "save1"))
  (bind _asbp_save_game (cast `/Game/Data/BP_SaveGame` _returnvalue))
  (set `self.SaveGameRef` _asbp_save_game)
  (`|ExecutionSequence`
    (:`then_0`
      (set `AC_NeuralNetwork.inputLayer` (`/Game/Data/BP_SaveGame.MoveRightNetworkInput` _savegameref) _nn_move_right)
      (set `AC_NeuralNetwork.hiddenLayer` (`/Game/Data/BP_SaveGame.MoveRightNetworkHidden` _savegameref) _nn_move_right)
      (set `AC_NeuralNetwork.outputLayer` (`/Game/Data/BP_SaveGame.MoveRightNetworkOutput` _savegameref) _nn_move_right)
      (set `AC_NeuralNetwork.expectedValue` (`/Game/Data/BP_SaveGame.MoveRightNetworkExpected` _savegameref) _nn_move_right))
    (:`then_1`
      (set `AC_NeuralNetwork.inputLayer` (`/Game/Data/BP_SaveGame.JumpRightNetworkInput` _savegameref) _nn_jump_right)
      (set `AC_NeuralNetwork.hiddenLayer` (`/Game/Data/BP_SaveGame.JumpRightNetworkHidden` _savegameref) _nn_jump_right)
      (set `AC_NeuralNetwork.outputLayer` (`/Game/Data/BP_SaveGame.JumpRightNetworkOutput` _savegameref) _nn_jump_right)
      (set `AC_NeuralNetwork.expectedValue` (`/Game/Data/BP_SaveGame.JumpRightNetworkExpected` _savegameref) _nn_jump_right))
    (:`then_2`
      (set `AC_NeuralNetwork.inputLayer` (`/Game/Data/BP_SaveGame.MoveLeftNetworkInput` _savegameref) _nn_move_left)
      (set `AC_NeuralNetwork.hiddenLayer` (`/Game/Data/BP_SaveGame.MoveLeftNetworkHidden` _savegameref) _nn_move_left)
      (set `AC_NeuralNetwork.outputLayer` (`/Game/Data/BP_SaveGame.MoveLeftNetworkOutput` _savegameref) _nn_move_left)
      (set `AC_NeuralNetwork.expectedValue` (`/Game/Data/BP_SaveGame.MoveLeftNetworkExpected` _savegameref) _nn_move_left))
    (:`then_3`
      (set `AC_NeuralNetwork.inputLayer` (`/Game/Data/BP_SaveGame.JumpLeftNetworkInput` _savegameref) _nn_jump_left)
      (set `AC_NeuralNetwork.hiddenLayer` (`/Game/Data/BP_SaveGame.JumpLeftNetworkHidden` _savegameref) _nn_jump_left)
      (set `AC_NeuralNetwork.outputLayer` (`/Game/Data/BP_SaveGame.JumpLeftNetworkOutput` _savegameref) _nn_jump_left)
      (set `AC_NeuralNetwork.expectedValue` (`/Game/Data/BP_SaveGame.JumpLeftNetworkExpected` _savegameref) _nn_jump_left))))

(event `AddAttemptByTime`
  (bind _gameinstanceref (`self.GameInstanceRef`))
  (bind (_leveldata_neuralnetworktype _leveldata_totaltimetocompletelevel _leveldata_timetocompletelevel _leveldata_totalattemptstocompletelevel _leveldata_numberofresetsbytime _leveldata_numberofresetsbydeath) (break `/Game/Data/DataCollection/S_PerLevelData` (`/Game/Data/BP_GameInstance.LevelData` _gameinstanceref)))
  ;[1 1 1 1 32] LEVEL DATA AND STATISTICS
  (set `/Game/Data/BP_GameInstance.LevelData` (make `/Game/Data/DataCollection/S_PerLevelData` _leveldata_neuralnetworktype _leveldata_totaltimetocompletelevel _leveldata_timetocompletelevel (+ _leveldata_totalattemptstocompletelevel 1) (+ _leveldata_numberofresetsbytime 1) _leveldata_numberofresetsbydeath) _gameinstanceref))

(event `SaveDataToFile`
  ;[1 1 1 1 32] LEVEL DATA AND STATISTICS
  (bind _returnvalue (`GameplayStatics.GetCurrentLevelName` true))
  (`/Game/Data/BP_GameInstance.SaveLevelData` (`self.GameInstanceRef`) _returnvalue))

(event `SaveNeuralNetworks`
  (params (NeuralNetworks :type "Array of AC_NeuralNetwork Object Reference"))
  (bind _savegameref (`self.SaveGameRef`))
  ;[1 1 1 1 32] SAVE AND LOAD FUNCTIONS
  ;;[1 1 1 1 24] SAVE THE NN DATA FROM AI TO SAVE
  (for (_array_element _array_index) NeuralNetworks
    (switch `int` _array_index
      (:`0`
        (bind _inputlayer (`AC_NeuralNetwork.inputLayer` _array_element))
        (set `/Game/Data/BP_SaveGame.MoveRightNetworkInput` _inputlayer _savegameref)
        (bind _hiddenlayer (`AC_NeuralNetwork.hiddenLayer` _array_element))
        (set `/Game/Data/BP_SaveGame.MoveRightNetworkHidden` _hiddenlayer _savegameref)
        (bind _outputlayer (`AC_NeuralNetwork.outputLayer` _array_element))
        (set `/Game/Data/BP_SaveGame.MoveRightNetworkOutput` _outputlayer _savegameref)
        (bind _expectedvalue (`AC_NeuralNetwork.expectedValue` _array_element))
        (set `/Game/Data/BP_SaveGame.MoveRightNetworkExpected` _expectedvalue _savegameref))
      (:`1`
        (set `/Game/Data/BP_SaveGame.JumpRightNetworkInput` _inputlayer _savegameref)
        (set `/Game/Data/BP_SaveGame.JumpRightNetworkHidden` _hiddenlayer _savegameref)
        (set `/Game/Data/BP_SaveGame.JumpRightNetworkOutput` _outputlayer _savegameref)
        (set `/Game/Data/BP_SaveGame.JumpRightNetworkExpected` _expectedvalue _savegameref))
      (:`2`
        (set `/Game/Data/BP_SaveGame.MoveLeftNetworkInput` _inputlayer _savegameref)
        (set `/Game/Data/BP_SaveGame.MoveLeftNetworkHidden` _hiddenlayer _savegameref)
        (set `/Game/Data/BP_SaveGame.MoveLeftNetworkOutput` _outputlayer _savegameref)
        (set `/Game/Data/BP_SaveGame.MoveLeftNetworkExpected` _expectedvalue _savegameref))
      (:`3`
        (set `/Game/Data/BP_SaveGame.JumpLeftNetworkInput` _inputlayer _savegameref)
        (set `/Game/Data/BP_SaveGame.JumpLeftNetworkHidden` _hiddenlayer _savegameref)
        (set `/Game/Data/BP_SaveGame.JumpLeftNetworkOutput` _outputlayer _savegameref)
        (set `/Game/Data/BP_SaveGame.JumpLeftNetworkExpected` _expectedvalue _savegameref))))
  (set `/Game/Data/BP_SaveGame.NNType` (`self.Neural Network Test`) _savegameref)
  (`GameplayStatics.SaveGameToSlot` _savegameref "save1"))

(fn `UserConstructionScript`)