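; AI character that learns to reach a goal along one axis by moving or jumping left or right, using four neural networks, one per action.
; A looping trial timer feeds hit and distance data from five fanned line traces into each network and performs the action whose output is nearest zero.
; Every fourth tick it retargets the last move's network by goal progress, backpropagates all four and saves them through the GameMode.
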(event `self.ReceiveBeginPlay`
  ;[1 1 1 1 32] On Spawn
  (bind _asgm_test_neural_network (cast `/Game/Levels/GM_TestNeuralNetwork` (`GameplayStatics.GetGameMode`)))
  (bind _output_get (set `self.Gamemode Ref` _asgm_test_neural_network))
  (`/Game/Levels/GM_TestNeuralNetwork.CheckSaveGame` _output_get self))

(event `InitializeAI`
  (params (Type :type "E_NeuralNetwork Enum" :default "E_Sigmoid"))
  (bind _nn_move_right (`self.NN_Move_Right`))
  (bind _nn_jump_left (`self.NN_Jump_Left`))
  (bind _nn_jump_right (`self.NN_Jump_Right`))
  (bind _nn_move_left (`self.NN_Move_Left`))
  ;[1 1 1 1 32] Initialize Neural Networks
  (`AC_NeuralNetwork.InitNeuralNetwork` _nn_move_right 10 7 1 0.5 Type)
  (`KismetArrayLibrary.Array_Add` (`self.NeuralNetworks`) _nn_move_right)
  (`AC_NeuralNetwork.InitNeuralNetwork` _nn_jump_right 10 7 1 0.5 Type)
  (`KismetArrayLibrary.Array_Add` (`self.NeuralNetworks`) _nn_jump_right)
  (`AC_NeuralNetwork.InitNeuralNetwork` _nn_move_left 10 7 1 0.5 Type)
  (`KismetArrayLibrary.Array_Add` (`self.NeuralNetworks`) _nn_move_left)
  (`AC_NeuralNetwork.InitNeuralNetwork` _nn_jump_left 10 7 1 0.5 Type)
  (`KismetArrayLibrary.Array_Add` (`self.NeuralNetworks`) _nn_jump_left)
  (`KismetSystemLibrary.PrintString` "INIT AI"))

(event `RunNNTrial`
  ;[1 1 1 1 32] Start Trial
  (`self.calcDisToGoal`)
  (bind _returnvalue (`KismetSystemLibrary.K2_SetTimerDelegate` (delegate `TrialLoop`) 0.75 true))
  (set `self.NNRunTimer` _returnvalue))

(event `TrialLoop`
  ;[1 1 1 1 32] Game loop
  (if (== (`self.moveCount`) 3)
    (`self.BackProp`)
    (set `self.moveCount` 0)
    (`/Game/Levels/GM_TestNeuralNetwork.SaveNeuralNetworks` (`self.Gamemode Ref`) (`self.NeuralNetworks`))
    (else
      (`self.FWDProp`)
      (`self.ChooseMovement`)
      (`KismetArrayLibrary.Array_Clear` (`self.inputValues`))
      (set `self.moveCount` (+ 1 (`self.moveCount`))))))

(event `FinalSaveBeforeReset`
  ;[1 1 1 1 32] Backprop and save NN before level restart
  (`/Game/Levels/GM_TestNeuralNetwork.SaveNeuralNetworks` (`self.Gamemode Ref`) (`self.NeuralNetworks`)))

(event `FWDProp`
  (bind _inputvalues (`self.inputValues`))
  ;[1 1 1 1 32] Send Line Trace as Inputs to NNs
  (`self.CreateLineTraces`)
  (for _array_element (`self.Input Line Traces`)
    (bind (_bblockinghit _binitialoverlap _time _distance _location _impactpoint) (`GameplayStatics.BreakHitResult` _array_element))
    (`KismetArrayLibrary.Array_Add` _inputvalues (`KismetMathLibrary.Conv_BoolToDouble` _bblockinghit))
    (`KismetArrayLibrary.Array_Add` _inputvalues (`KismetMathLibrary.NormalizeToRange` (`KismetMathLibrary.Vector_Distance` (`self.K2_GetActorLocation`) _impactpoint) 0.0 1004.309504)))
  (for (_array_element_2 _array_index) (`self.NeuralNetworks`)
    (bind _returnvalue (`AC_NeuralNetwork.FwdPropNN` _array_element_2 (`self.inputValues`)))
    (`KismetArrayLibrary.Array_Set` (`self.outputValues`) _array_index _returnvalue)))

(event `ChooseMovement`
  (bind (_value _index) (`self.getClosestToZero` (`self.outputValues`)))
  ;[1 1 1 1 32] Forward prop through each NN and get output; Using that output move the AI
  (`KismetArrayLibrary.Array_Set` (`self.movesMade`) (`self.moveCount`) (make `/Game/AI/S_PreviousMoves` _index _value) true)
  (switch `int` _index
    (:`Default`
      (`KismetSystemLibrary.PrintString` "Move Right" false true (struct :`G` 0.66 :`B` 1.0 :`A` 1.0) 5.0 :!label _label)
      (set `self.moveDir` 1.0)
      (`self.StartMovement` false :!label _label_2))
    (:`0`
      (goto _label))
    (:`1`
      (`KismetSystemLibrary.PrintString` "Jump Right" false true (struct :`G` 0.66 :`B` 1.0 :`A` 1.0) 5.0)
      (set `self.moveDir` 1.0)
      (`self.StartMovement` true :!label _label_3))
    (:`2`
      (`KismetSystemLibrary.PrintString` "Move Left" false true (struct :`G` 0.66 :`B` 1.0 :`A` 1.0) 5.0)
      (set `self.moveDir` -1.0)
      (goto _label_2))
    (:`3`
      (`KismetSystemLibrary.PrintString` "Jump Left" false true (struct :`G` 0.66 :`B` 1.0 :`A` 1.0) 5.0)
      (set `self.moveDir` -1.0)
      (goto _label_3))))

(event `BackProp`
  (bind _movesmade (`self.movesMade`))
  (bind _output (`|GetArrayItem` (`self.NeuralNetworks`) (`.move_8_A03D7B6E4565DFC50315B29F165E9860` (break `/Game/AI/S_PreviousMoves` (`|GetArrayItem` _movesmade (`KismetArrayLibrary.Array_LastIndex` _movesmade))))))
  ;[1 1 1 1 32] Back prop through each NN
  (bind (_need_to_make_better_moves _returnvalue) (`self.evaluateDisToGoal`))
  (set `self.oldDistance` _returnvalue)
  (if _need_to_make_better_moves
    (set `AC_NeuralNetwork.expectedValue` 100.0 _output)
    (else
      (set `AC_NeuralNetwork.expectedValue` 0.0 _output)))
  (for _array_element (`self.NeuralNetworks`)
    (`AC_NeuralNetwork.BackPropNN` _array_element)))

(event `CreateLineTraces`
  (bind _returnvalue (`self.K2_GetActorLocation`))
  ;[1 1 1 1 32] Create Line Traces for inputs
  (for _index (range 5)
    (bind _outhit (`KismetSystemLibrary.LineTraceSingle` :`Start` _returnvalue :`End` (+ _returnvalue (* (`KismetMathLibrary.RotateAngleAxis` (`SceneComponent.GetRightVector` (`self.Mesh`)) (select `int` _index :`0` -67.5 :`1` -45.0 :`2` 0.0 :`3` 45.0 :`4` 67.5 :!type "Float (single-precision)") (1.0 0.0 0.0)) 500.0)) :`TraceChannel` "TraceTypeQuery1" :`DrawDebugType` "ForDuration" :`DrawTime` 0.75))
    (`KismetArrayLibrary.Array_Set` (`self.Input Line Traces`) _index _outhit)))

(event `StartMovement`
  (params (mustJump :type Boolean))
  ;[1 1 1 1 32] Movement Code for AI
  (bind _returnvalue (`KismetSystemLibrary.K2_SetTimerDelegate` (delegate `Move`) 0.01 true))
  (if mustJump
    (`KismetSystemLibrary.Delay` 0.25)
    (`self.Jump`))
  (`KismetSystemLibrary.Delay` 0.75)
  (`KismetSystemLibrary.K2_ClearAndInvalidateTimerHandle` _returnvalue))

(event `BackpropFromDeath`
  (bind _movesmade (`self.movesMade`))
  ;[1 1 1 1 32] Death Backprop
  (set `AC_NeuralNetwork.expectedValue` 0.0 (`|GetArrayItem` (`self.NeuralNetworks`) (`.move_8_A03D7B6E4565DFC50315B29F165E9860` (break `/Game/AI/S_PreviousMoves` (`|GetArrayItem` _movesmade (`KismetArrayLibrary.Array_LastIndex` _movesmade))))))
  (for _array_element (`self.NeuralNetworks`)
    (`AC_NeuralNetwork.BackPropNN` _array_element)))

(event `Move`
  ;[1 1 1 1 32] Movement Code for AI
  (`self.AddMovementInput` (0.0 1.0 0.0) (`self.moveDir`)))

(fn `calcDisToGoal`
  (set `self.oldDistance` (`KismetMathLibrary.Vector_Distance` (`self.K2_GetActorLocation`) (`self.goalLocation`))))

(fn `evaluateDisToGoal`
  (returns (`Need to make better moves` :type Boolean) (ReturnValue :type "Float (double-precision)"))
  (bind _returnvalue (`KismetMathLibrary.Vector_Distance` (`self.K2_GetActorLocation`) (`self.goalLocation`)))
  (if (<= (`self.oldDistance`) _returnvalue)
    (`KismetSystemLibrary.PrintString` "Need to make better moves")
    (return true _returnvalue)
    (else
      (`KismetSystemLibrary.PrintString` "Have made okay moves")
      (return false _returnvalue))))

(fn `getClosestToZero`
  (params (outputValues :type "Array of Float (double-precision)"))
  (returns (value :type "Float (double-precision)") (index :type Integer))
  (locals (minValue :type "Float (double-precision)" :default 100000000.0) (minIndex :type Integer :default -1))
  (for (_array_element _array_index) outputValues
    (if (< (`KismetMathLibrary.Abs` _array_element) (`local.minValue`))
      (set `local.minValue` _array_element)
      (set `local.minIndex` _array_index)))
  (return (`local.minValue`) (`local.minIndex`)))

(fn `setGoalLocation`
  (params (goalLocation :type "Vector Structure"))
  (set `self.goalLocation` goalLocation))

(fn `UserConstructionScript`)